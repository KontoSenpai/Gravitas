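; CubeFire is a fire cube Blueprint that melts CubeFrozen and CubeIce actors it touches.
; Three per-axis overlap components (X, Y, Z) each wait half a second, then, unless Input is set, call Melt on the overlapped cube.
; It stores the returned position (plus a reference for frozen cubes), flags which type melted and sets Melt to true; this graph does not act on those values further.
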(event `self.OverlapDetectionZ.OnComponentBeginOverlap`
  (params (OtherActor :type "Actor Object Reference") (OtherComp :type "PrimitiveComponent Object Reference") (OtherBodyIndex :type Integer) (bFromSweep :type Boolean) (SweepResult :type "EngineTypes.HitResult Structure (by ref)"))
  (bind _returnvalue (`GameplayStatics.GetObjectClass` OtherActor))
  ;[1 1 1] Collision sur Z
  (`KismetSystemLibrary.Delay` 0.5)
  (if (`self.Input`)
    _
    (elif (== _returnvalue "/Game/Blueprints/Cubes/cubeFrozen.cubeFrozen_C")
      (bind _ascube_frozen (cast `/Game/Blueprints/Cubes/cubeFrozen` OtherActor))
      (bind (_old_position _ref) (`/Game/Blueprints/Cubes/cubeFrozen.Melt` _ascube_frozen))
      (set `self.PosMelt` _old_position)
      (set `self.Ref` _ref)
      (set `self.IceOrFrozen` 0 :!label _label)
      (set `self.melt` true :!label _label_2)
      (elif (== _returnvalue "/Game/Blueprints/Cubes/CubeIce.CubeIce_C")
        (bind _ascube_ice (cast `/Game/Blueprints/Cubes/CubeIce` OtherActor))
        (bind _oldposition (`/Game/Blueprints/Cubes/CubeIce.Melt` _ascube_ice))
        (set `self.PosMelt` _oldposition)
        (set `self.IceOrFrozen` 1 :!label _label_3)
        (goto _label_2)))))

(event `self.OverlapDetectionY.OnComponentBeginOverlap`
  (params (OtherActor :type "Actor Object Reference") (OtherComp :type "PrimitiveComponent Object Reference") (OtherBodyIndex :type Integer) (bFromSweep :type Boolean) (SweepResult :type "EngineTypes.HitResult Structure (by ref)"))
  (bind _returnvalue (`GameplayStatics.GetObjectClass` OtherActor))
  ;[1 1 1] Collision sur Y
  (`KismetSystemLibrary.Delay` 0.5)
  (if (`self.Input`)
    _
    (elif (== _returnvalue "/Game/Blueprints/Cubes/cubeFrozen.cubeFrozen_C")
      (bind _ascube_frozen (cast `/Game/Blueprints/Cubes/cubeFrozen` OtherActor))
      (bind (_old_position _ref) (`/Game/Blueprints/Cubes/cubeFrozen.Melt` _ascube_frozen))
      (set `self.PosMelt` _old_position)
      (set `self.Ref` _ref)
      (goto _label)
      (elif (== _returnvalue "/Game/Blueprints/Cubes/CubeIce.CubeIce_C")
        (bind _ascube_ice (cast `/Game/Blueprints/Cubes/CubeIce` OtherActor))
        (bind _oldposition (`/Game/Blueprints/Cubes/CubeIce.Melt` _ascube_ice))
        (set `self.PosMelt` _oldposition)
        (goto _label_3)))))

(event `self.OverlapDetectionX.OnComponentBeginOverlap`
  (params (OtherActor :type "Actor Object Reference") (OtherComp :type "PrimitiveComponent Object Reference") (OtherBodyIndex :type Integer) (bFromSweep :type Boolean) (SweepResult :type "EngineTypes.HitResult Structure (by ref)"))
  (bind _returnvalue (`GameplayStatics.GetObjectClass` OtherActor))
  ;[1 1 1] Collision sur X
  (`KismetSystemLibrary.Delay` 0.5)
  (if (`self.Input`)
    _
    (elif (== _returnvalue "/Game/Blueprints/Cubes/cubeFrozen.cubeFrozen_C")
      (bind _ascube_frozen (cast `/Game/Blueprints/Cubes/cubeFrozen` OtherActor))
      (bind (_old_position _ref) (`/Game/Blueprints/Cubes/cubeFrozen.Melt` _ascube_frozen))
      (set `self.PosMelt` _old_position)
      (set `self.Ref` _ref)
      (goto _label)
      (elif (== _returnvalue "/Game/Blueprints/Cubes/CubeIce.CubeIce_C")
        (bind _ascube_ice (cast `/Game/Blueprints/Cubes/CubeIce` OtherActor))
        (bind _oldposition (`/Game/Blueprints/Cubes/CubeIce.Melt` _ascube_ice))
        (set `self.PosMelt` _oldposition)
        (goto _label_3)))))

(fn `UserConstructionScript`
  (set `self.Input` false)
  (set `self.MatIndex` 0))