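; Frozen cube actor that can melt into a regular Cube, intended for contact with a fire cube.
; Melt hides it, spawns the Cube at a fixed offset from its location, and returns its old transform and the new cube reference.
; DestroyActor follows the return in a Sequence, so it likely never runs.
; Contact detection is not in this Blueprint; BeginPlay and construction only call the parent.
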(event `self.ReceiveBeginPlay`
  (`parent.ReceiveBeginPlay`))

(fn `Melt`
  (returns (`old position` :type "Object.Transform Structure") (ref :type "/Game/Blueprints/Cubes/Cube Object Reference"))
  ;[1 1 1] Fondre au contact d'un cube de feu
  (`SceneComponent.SetVisibility` false)
  (bind _returnvalue (`|SpawnActorFromClass` "/Game/Blueprints/Cubes/Cube.Cube_C" (`KismetMathLibrary.Conv_VectorToTransform` (+ (`self.K2_GetActorLocation`) (50.0 -50.0 50.0)))))
  (`|ExecutionSequence`
    (:`then_0`
      (return (`self.GetTransform`) _returnvalue))
    (:`then_1`
      (`self.K2_DestroyActor`))))

(fn `UserConstructionScript`
  (`parent.UserConstructionScript`))