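; Automaton character blueprint with a camera that hides obstructing static meshes, toggleable input and obstacle detection.
; A looping timer traces from the camera to hide the hit mesh, paused while the box overlaps a trigger volume, and sets Walk from velocity.
; SwitchInputAutomate swaps glow material and axis locks with the input state.
; CubeDetect classifies a downward sphere trace by distance into climb, top-block or bottom-block flags.
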(event `self.Box.OnComponentBeginOverlap`
  (params (OtherActor :type "Actor Object Reference") (OtherComp :type "PrimitiveComponent Object Reference") (OtherBodyIndex :type Integer) (bFromSweep :type Boolean) (SweepResult :type "EngineTypes.HitResult Structure (by ref)"))
  ;[1 1 1] Camera masquée
  (cast `TriggerVolume` OtherActor)
  (set `self.StopDisappear` true))

(event `self.Box.OnComponentEndOverlap`
  (params (OtherActor :type "Actor Object Reference") (OtherComp :type "PrimitiveComponent Object Reference") (OtherBodyIndex :type Integer))
  ;[1 1 1] Camera masquée
  (cast `TriggerVolume` OtherActor)
  (set `self.StopDisappear` false))

(event `self.ReceiveBeginPlay`
  (`KismetSystemLibrary.K2_SetTimer` null "hey" 0.1 true))

(event `hey`
  (bind _sma (`self.SMA`))
  (bind _camera (`self.Camera`))
  ;[1 1 1] Hey
  (`|ExecutionSequence`
    (:`then_0`
      (if (`KismetSystemLibrary.IsValid` _sma)
        (`self.SetActorHiddenInGame` _sma false))
      (if (not (`self.StopDisappear`))
        (bind (_outhit _returnvalue) (`KismetSystemLibrary.LineTraceSingleForObjects` (* (`SceneComponent.K2_GetComponentLocation` _camera) 500.0) (* (`KismetMathLibrary.GetForwardVector` (`SceneComponent.K2_GetComponentRotation` _camera)) 5000.0) (`|MakeArray` "ObjectTypeQuery1" :!type "EngineTypes.EObjectTypeQuery Enum")))
        (if _returnvalue
          (bind _asstatic_mesh_actor (cast `StaticMeshActor` (`.HitActor` (`GameplayStatics.BreakHitResult` _outhit))))
          (bind _output_get (set `self.SMA` _asstatic_mesh_actor))
          (`self.SetActorHiddenInGame` _output_get true))))
    (:`then_1`
      (if (!= (`self.GetVelocity`) (0.0 0.0 0.0))
        (set `self.Walk` true)
        (else
          (set `self.Walk` false))))))

(fn `CubeDetect`
  (bind _returnvalue (`SceneComponent.K2_GetComponentLocation` (`self.Sphere`)))
  ;[1 1 1] Réinitialisation des valeurs a défaut
  (set `self.Climb` false)
  (set `self.botBlock` false)
  (set `self.topBlock` false)
  (bind _outhit (`KismetSystemLibrary.LineTraceSingleForObjects` _returnvalue (- _returnvalue (0.0 0.0 1000.0)) (`|MakeArray` "ObjectTypeQuery1" :!type "EngineTypes.EObjectTypeQuery Enum")))
  (bind _returnvalue_2 (`KismetMathLibrary.VSize` (- _returnvalue (`.ImpactPoint` (`GameplayStatics.BreakHitResult` _outhit)))))
  ;[1 1 1] Assignation des valeurs de l'automate selon la longueur sphere-objet
  (`/Engine/EditorBlueprintResources/StandardMacros.CompareFloat` _returnvalue_2 200.0
    (:`>`
      (`/Engine/EditorBlueprintResources/StandardMacros.CompareFloat` _returnvalue_2 350.0
        (:`>`
          (set `self.botBlock` true))))
    (:`==`
      (`/Engine/EditorBlueprintResources/StandardMacros.CompareFloat` _returnvalue_2 90.0 :!label _label
        (:`==`
          (set `self.Climb` true :!label _label_2))
        (:`<`
          (if (`KismetMathLibrary.NearlyEqual_FloatFloat` _returnvalue_2 0.0 20.0)
            (set `self.topBlock` true)
            (else
              (goto _label_2))))))
    (:`<`
      (goto _label))))

(fn `SwitchInputAutomate`
  (bind _mesh (`self.Mesh`))
  (if (`self.Input`)
    (set `self.Input` false)
    (`PrimitiveComponent.SetMaterial` _mesh 0 "/Game/Materials/Interactif/M_gold_automate.M_gold_automate")
    (`PrimitiveComponent.SetLockedAxis` "Y")
    (`PrimitiveComponent.SetLockedAxis` "X")
    (`PrimitiveComponent.SetLockedAxis` "Z")
    (else
      (set `self.Input` true)
      (`PrimitiveComponent.SetMaterial` _mesh 0 "/Game/Materials/Interactif/M_Gold_Automate_Glow.M_Gold_Automate_Glow")
      (`PrimitiveComponent.SetLockedAxis` "None"))))

(fn `UserConstructionScript`
  (bind _camera (`self.Camera`))
  (`SceneComponent.K2_SetWorldLocation` (`self.SpringArm`) (0.0 0.0 0.0) false)
  (bind _outhit (`KismetSystemLibrary.LineTraceSingleForObjects` (`SceneComponent.K2_GetComponentLocation` _camera) (* (`KismetMathLibrary.GetForwardVector` (`SceneComponent.K2_GetComponentRotation` _camera)) 5000.0) (`|MakeArray` "ObjectTypeQuery1" :!type "EngineTypes.EObjectTypeQuery Enum")))
  (bind _asstatic_mesh_actor (cast `StaticMeshActor` (`.HitActor` (`GameplayStatics.BreakHitResult` _outhit))))
  (set `self.SMA` _asstatic_mesh_actor))