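; Interactive moving element, such as a door, that slides between an initial and end location when a switch event fires.
; The Motion timeline drives a lerp of the actor's relative location, from the position captured in the construction script to EndLocation.
; With KeepState, it plays forward and locks as Activated when finished; otherwise each interaction toggles between playing and reversing.
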(event `self.InteractWithSwitch`
  (params (KeepState :type Boolean))
  ;[1 1 1] Move the Door
  (set `self.Forward` (not (`self.Forward`)))
  (if KeepState
    (if (not (`self.Activated`))
      (bind (_direction _driver) (`Timeline|Motion` :!label _label)
        (:`Update`
          (`self.K2_SetActorRelativeLocation` (`KismetMathLibrary.VLerp` (`self.Initial Location`) (`self.End Location`) _driver)))
        (:`Finished`
          (if KeepState
            (set `self.Activated` true)))))
    (elif (`self.Forward`)
      (goto _label)
      (else
        (goto _label :!via `Reverse`)))))

(event `self.ReceiveBeginPlay`)

(event `self.ReceiveActorBeginOverlap`
  (params (OtherActor :type "Actor Object Reference")))

(event `self.ReceiveTick`
  (params (DeltaSeconds :type "Float (single-precision)")))

(fn `UserConstructionScript`
  (bind _returnvalue (`self.K2_GetActorLocation`))
  (`parent.UserConstructionScript`)
  (`self.K2_SetActorLocation` _returnvalue)
  (set `self.Initial Location` _returnvalue))