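; Trigger-volume switch that signals a list of linked actors when components tagged "overlapSwitch" enter or leave it.
; Both overlap events share one path, sending InteractWithSwitchMessage with KeepState to SelectedActors that implement Interface_ActivatedBySwitch.
; Messages fire for qualifying overlapping actors, plus an extra pass for "automan"-tagged components when InteractWithAutomate is set.
; The construction script applies scale and optional mesh and material overrides.
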(event `self.TriggerVolume.OnComponentEndOverlap`
  (params (OtherActor :type "Actor Object Reference") (OtherComp :type "PrimitiveComponent Object Reference") (OtherBodyIndex :type Integer))
  (if (`ActorComponent.ComponentHasTag` OtherComp "overlapSwitch")
    (if (`self.Interact with Automate`)
      (`|ExecutionSequence` :!label _label
        (:`then_0`
          (if (`ActorComponent.ComponentHasTag` (stale `self.TriggerVolume.OnComponentBeginOverlap` OtherComp) "automan")
            (for _array_element (`self.Selected Actors`) :!label _label_2
              (if (`KismetSystemLibrary.DoesImplementInterface` _array_element "/Game/Blueprints/InteractiveElements/Interface_ActivatedBySwitch.Interface_ActivatedBySwitch_C")
                (message `/Game/Blueprints/InteractiveElements/Interface_ActivatedBySwitch.InteractWithSwitch` _array_element (`self.Keep State`))))))
        (:`then_1`
          (for _array_element_2 (`PrimitiveComponent.GetOverlappingActors` null) :!label _label_3
            (if (`KismetArrayLibrary.Array_Contains` (`self.Overlapping Actors`) _array_element_2)
              (goto _label_2)))))
      (else
        (goto _label_3)))))

(event `self.TriggerVolume.OnComponentBeginOverlap`
  (params (OtherActor :type "Actor Object Reference") (OtherComp :type "PrimitiveComponent Object Reference") (OtherBodyIndex :type Integer) (bFromSweep :type Boolean) (SweepResult :type "EngineTypes.HitResult Structure (by ref)"))
  (if (`ActorComponent.ComponentHasTag` OtherComp "overlapSwitch")
    (if (`self.Interact with Automate`)
      (goto _label)
      (else
        (goto _label_3)))))

(fn `UserConstructionScript`
  (`SceneComponent.SetRelativeScale3D` (`KismetMathLibrary.Conv_DoubleToVector` (`self.3D Scale`)))
  (`|ExecutionSequence`
    (:`then_0`
      (if (!= (`self.Switch Mesh Override`) null)
        (`StaticMeshComponent.SetStaticMesh` (`self.Switch Mesh Override`))))
    (:`then_1`
      (if (!= (`self.Switch Material Override`) null)
        (`PrimitiveComponent.SetMaterial` 2 (`self.Switch Material Override`))))))