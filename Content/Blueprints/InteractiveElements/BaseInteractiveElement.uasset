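; Base actor Blueprint for interactive elements, exposing an empty Action function that presumably child classes override.
; The Construction Script applies a configurable relative 3D scale, then swaps in an optional mesh and a slot-zero material when those override variables are set.
; The event graph holds only disabled placeholder events, so the base has no runtime behavior of its own.
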(event `self.ReceiveBeginPlay`)

(event `self.ReceiveActorBeginOverlap`
  (params (OtherActor :type "Actor Object Reference")))

(event `self.ReceiveTick`
  (params (DeltaSeconds :type "Float (single-precision)")))

(fn `Action`)

(fn `UserConstructionScript`
  (`SceneComponent.SetRelativeScale3D` (`self.3D Scale`))
  (`|ExecutionSequence`
    (:`then_0`
      (if (!= (`self.Component Mesh Override`) null)
        (`StaticMeshComponent.SetStaticMesh` (`self.Component Mesh Override`))))
    (:`then_1`
      (if (!= (`self.Component Material Override`) null)
        (`PrimitiveComponent.SetMaterial` 0 (`self.Component Material Override`))))))