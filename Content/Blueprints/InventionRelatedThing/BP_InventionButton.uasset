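; BP_InventionButton is a button actor for an invention system that knows its integer cell on a 3D grid.
; InitializeInventionButton derives X, Y and Z by flooring its offset from an Origin actor divided by the grid unit, and GetCoord returns them.
; Activate sets Activated true only for the button at cell (0,0,0), and turns off visibility regardless of the result.
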(event `self.ReceiveBeginPlay`)

(event `self.ReceiveActorBeginOverlap`
  (params (OtherActor :type "Actor Object Reference")))

(event `self.ReceiveTick`
  (params (DeltaSeconds :type "Float (single-precision)")))

(fn `Activate`
  (set `self.Activated` (and (== 0 (`self.X`)) (== 0 (`self.Y`)) (== 0 (`self.Z`))))
  (`SceneComponent.SetVisibility` false))

(fn `GetCoord`
  (returns (X :type Integer) (Y :type Integer) (Z :type Integer))
  (return (`self.X`) (`self.Y`) (`self.Z`)))

(fn `InitializeInventionButton`
  (params (Origin :type "/Game/Blueprints/GridRelatedThing/BP_GridMarker Object Reference") (GridUnit :type "Float (double-precision)" :default 0.0))
  (bind (_returnvalue_x _returnvalue_y _returnvalue_z) (`KismetMathLibrary.BreakVector` (`self.K2_GetActorLocation` Origin)))
  (bind (_returnvalue_x_2 _returnvalue_y_2 _returnvalue_z_2) (`KismetMathLibrary.BreakVector` (`self.K2_GetActorLocation`)))
  (set `self.X` (`KismetMathLibrary.FFloor` (/ (- _returnvalue_x_2 _returnvalue_x) GridUnit)))
  (set `self.Y` (`KismetMathLibrary.FFloor` (/ (- _returnvalue_y_2 _returnvalue_y) GridUnit)))
  (set `self.Z` (`KismetMathLibrary.FFloor` (/ (- _returnvalue_z_2 _returnvalue_z) GridUnit))))

(fn `UserConstructionScript`)